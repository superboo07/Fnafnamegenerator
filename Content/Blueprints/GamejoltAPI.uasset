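; GamejoltAPI sets up the Game Jolt connection and restores saved player data when its Init event fires.
; It initializes the API with a hardcoded game ID and private key, then logs in automatically using credentials from an existing LoginSave.
; It also copies custom name lists and related settings from CustomNamesSave into its variables.
; When either save slot is missing, it creates a fresh save object in memory without writing it.
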(event EventInit
  (bind _returnvalue (Class|GameJolt|Initialize 553598 "ff58c8e4173e0c384bc8288ff68ea16b"))
  (Variables|Default|SetGamejoltAPI _returnvalue)
  (Utilities|FlowControl|Sequence
    (:then_0
      (bind _returnvalue_2 (SaveGame|DoesSaveGameExist "game"))
      (if _returnvalue_2
        (bind _returnvalue_3 (SaveGame|LoadGamefromSlot "game"))
        (bind _output_get (Variables|Default|SetSave _returnvalue_3))
        (bind _aslogin_save (Utilities|Casting|CastToLoginSave _output_get))
        (bind _output_get_2 (Variables|Default|SetSavecasted _aslogin_save))
        (|Login (Variables|Default|GetGamejoltAPI) (Variables|/Game/LoginSave.LoginSave_C|GetUsername _output_get_2) (Variables|/Game/LoginSave.LoginSave_C|GetKey _output_get_2)
          (:Success
            (Development|PrintString "HAHA")
            (Variables|Default|SetIs_Loggedin true)))
        (else
          (bind _returnvalue_4 (SaveGame|CreateSaveGameObject "/Game/LoginSave.LoginSave_C"))
          (bind _output_get_3 (Variables|Default|SetSave _returnvalue_4))
          (bind _aslogin_save_2 (Utilities|Casting|CastToLoginSave _output_get_3))
          (Variables|Default|SetSavecasted _aslogin_save_2))))
    (:then_1
      (bind _returnvalue_5 (SaveGame|DoesSaveGameExist "custom"))
      (if _returnvalue_5
        (bind _returnvalue_6 (SaveGame|LoadGamefromSlot "custom"))
        (bind _ascustom_names_save (Utilities|Casting|CastToCustomNamesSave _returnvalue_6))
        (bind _output_get_4 (Variables|Default|SetCustomSave _ascustom_names_save))
        (Variables|Default|SetNames (Variables|/Game/CustomNamesSave.CustomNamesSave_C|GetNames _output_get_4))
        (Variables|Default|SetNameTypes (Variables|/Game/CustomNamesSave.CustomNamesSave_C|GetSet _output_get_4))
        (Variables|Default|SetAliasNames (Variables|/Game/CustomNamesSave.CustomNamesSave_C|GetAliasSet _output_get_4))
        (Variables|Default|SetCanHaveBeforeName (Variables|/Game/CustomNamesSave.CustomNamesSave_C|GetCanhavebeforename _output_get_4))
        (else
          (bind _returnvalue_7 (SaveGame|CreateSaveGameObject "/Game/CustomNamesSave.CustomNamesSave_C"))
          (Variables|Default|SetCustomSave _returnvalue_7))))))